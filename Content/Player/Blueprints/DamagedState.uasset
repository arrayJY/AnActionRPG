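; Anim notify state that marks the player character as damaged for the span it covers in an animation.
; On begin and end it casts the mesh owner to PlayerCharacter and sets IsDamaged to true, then back to false.
; Both events also print a debug string, before the cast.
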(fn ReceivedNotifyBegin
  (params (MeshComp :type Skeletal%20Mesh%20Component%20Object%20Reference) (Animation :type Anim%20Sequence%20Base%20Object%20Reference) (TotalDuration :type Float%20%28single-precision%29))
  (Development|PrintString 0 "Begin")
  (bind _asplayer_character (Utilities|Casting|CastToPlayerCharacter (Components|GetOwner MeshComp)))
  (Variables|/Script/FinalProject2.BasePlayerCharacter|SetIsDamaged _asplayer_character true)
  (return false))

(fn ReceivedNotifyEnd
  (params (MeshComp :type Skeletal%20Mesh%20Component%20Object%20Reference) (Animation :type Anim%20Sequence%20Base%20Object%20Reference))
  (Development|PrintString 0 "End")
  (bind _asplayer_character (Utilities|Casting|CastToPlayerCharacter (Components|GetOwner MeshComp)))
  (Variables|/Script/FinalProject2.BasePlayerCharacter|SetIsDamaged _asplayer_character false)
  (return false))
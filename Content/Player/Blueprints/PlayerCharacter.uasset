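; Player character Blueprint that deals melee-style damage through a HitBox component.
; The HitBox starts with collision disabled at BeginPlay, and nothing in this file re-enables it.
; On overlap, it applies fixed damage to the other actor unless that actor is the HitBox owner, and prints a debug string.
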(event OnComponentBeginOverlap(HitBox)
  (params (OverlappedComponent :type Primitive%20Component%20Object%20Reference) (OtherActor :type Actor%20Object%20Reference) (OtherComp :type Primitive%20Component%20Object%20Reference) (OtherBodyIndex :type Integer) (bFromSweep :type Boolean) (SweepResult :type Hit%20Result%20Structure%20%28by%20ref%29))
  (Variables|Default|SetHitWeapon OverlappedComponent)
  (Variables|Default|SetTarget OtherActor)
  (Variables|Default|SetAttacker (Components|GetOwner (Variables|Default|GetHitWeapon)))
  (if (not (== (Variables|Default|GetAttacker) (Variables|Default|GetTarget)))
    (Development|PrintString "Hello")
    (Game|Damage|ApplyDamage (Variables|Default|GetTarget) 1e+01 0 0)))

(event EventBeginPlay
  (Collision|SetCollisionEnabled (Variables|Default|GetHitBox) "NoCollision"))

(fn ConstructionScript)
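; Base character Blueprint that provides a world-space health bar, HUD updates and melee hit damage.
; SetHealthBar pushes health to the widget and, when valid, to the HUD reference, which also receives score through SetScoreText.
; Tick rotates the health bar to face the player camera.
; The HitBox starts without collision, and its overlaps apply fixed damage to actors other than its owner.
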(event OnComponentBeginOverlap(HitBox)
  (params (OverlappedComponent :type Primitive%20Component%20Object%20Reference) (OtherActor :type Actor%20Object%20Reference) (OtherComp :type Primitive%20Component%20Object%20Reference) (OtherBodyIndex :type Integer) (bFromSweep :type Boolean) (SweepResult :type Hit%20Result%20Structure%20%28by%20ref%29))
  ;[1 1 1] Melee Attack
  (bind _output_get (Variables|Default|SetWeapon OverlappedComponent))
  (Variables|Default|SetAttacker (Components|GetOwner _output_get))
  (Variables|Default|SetTarget OtherActor)
  (if (not (== (Variables|Default|GetAttacker) (Variables|Default|GetTarget)))
    (Game|Damage|ApplyDamage (Variables|Default|GetTarget) 1e+01 0 (Variables|Default|GetAttacker))))

(event EventSetScoreText
  (params (Val :type Integer))
  (bind _hudref (Variables|Default|GetHUDRef))
  ;[1 1 1] Update Score HUD
  (Utilities|IsValid _hudref
    (:Is%20Valid
      (Default|UpdateScore _hudref Val))))

(event EventSetHealthBar
  (params (Val :type Float%20%28single-precision%29))
  (bind _hudref (Variables|Default|GetHUDRef))
  ;[1 1 1] Update HealthBar and HUD
  (bind _ashealth_bar (Utilities|Casting|CastToHealthBar (UserInterface|GetUserWidgetObject (Variables|Default|GetHealthBar))))
  (Default|UpdateHealth _ashealth_bar Val)
  (Utilities|IsValid _hudref
    (:Is%20Valid
      (Default|UpdateHealth _hudref Val))))

(event EventTick
  (params (DeltaSeconds :type Float%20%28single-precision%29))
  (CallFunction|RotateHealthbartoPlayer))

(event EventBeginPlay
  (Collision|SetCollisionEnabled (Variables|Default|GetHitBox) "NoCollision"))

(fn ConstructionScript)

(fn RotateHealthbartoPlayer
  (Transformation|SetWorldRotation (Variables|Default|GetHealthBar) (Math|Rotator|FindLookatRotation (Transformation|GetWorldLocation (Variables|Default|GetHealthBar)) (Camera|GetCameraLocation (Game|GetPlayerCameraManager 0))) false false)
  (return))
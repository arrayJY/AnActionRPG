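; ArcherEnemyCharacter is the ranged archer enemy, which fires arrows as its attack.
; Forward and right movement inputs pass to shared common movement functions only while Animation.IsAttacking1 is false.
; StartAttack spawns an ArrowActor offset along the mesh's right vector, sets itself as owner, fires the arrow in that direction, then calls StartAttackCommon.
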(event Collision|EventActorBeginOverlap
  (params (OtherActor :type Actor%20Object%20Reference)))

(event EventTick
  (params (DeltaSeconds :type Float%20%28single-precision%29))
  (|CallParentFunction DeltaSeconds) ; 此节点被禁用，将不会被调用。\n从引脚连出引线来编译功能。
)

(event EventMoveForward
  (params (Value :type Float%20%28single-precision%29))
  (if (not (Variables|/Script/FinalProject2.PlayerAnimInstance|GetIsAttacking1 (Variables|Default|GetAnimation)))
    (Class|BasePlayerCharacter|MoveForwardCommon Value)))

(event EventMoveRight
  (params (Value :type Float%20%28single-precision%29))
  (if (not (Variables|/Script/FinalProject2.PlayerAnimInstance|GetIsAttacking1 (Variables|Default|GetAnimation)))
    (Class|BasePlayerCharacter|MoveRightCommon Value)))

(event EventBeginPlay)

(event EventStartAttack
  (bind _mesh (Variables|Character|GetMesh))
  (bind _returnvalue (Transformation|GetWorldRotation _mesh))
  (bind _returnvalue_2 (Math|Vector|GetRightVector _returnvalue))
  (bind _returnvalue_3 (Game|SpawnActorfromClass "/Script/FinalProject2.ArrowActor" (Math|Transform|MakeTransform (+ (.Location (Math|Transform|BreakTransform (Transformation|GetActorTransform))) (* _returnvalue_2 1e+02)) (Transformation|GetActorRotation)) "Undefined" 0 (Game|GetInstigator)))
  (Actor|SetOwner _returnvalue_3 self)
  (Class|ArrowActor|FireinDirection _returnvalue_3 _returnvalue_2)
  (Class|BasePlayerCharacter|StartAttackCommon))

(fn ConstructionScript
  (|CallParentFunction))